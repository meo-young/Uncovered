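; BP_Parent_Light is a parent light Blueprint for the office environment that gives its lights and lamp mesh a shared color and brightness control.
; The construction script scales every light component's intensity by IntensityMultiply, applies LightColor, and records each light in a map with a zero value.
; It also writes doubled IntensityMultiply and LightColor into the Lamp's default custom primitive data.
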(fn `UserConstructionScript`
  (bind _lamp (`self.Lamp`))
  (bind (_light_color_r _light_color_g _light_color_b _light_color_a) (break `LinearColor` (`self.Light Color`)))
  (bind _intensitymultiply (`self.IntensityMultiply`))
  (`BlueprintMapLibrary.Map_Clear` (`self.LightAndBaseIntensity`))
  (for _array_element (`self.K2_GetComponentsByClass` "/Script/Engine.LightComponent")
    (`BlueprintMapLibrary.Map_Add` (`self.LightAndBaseIntensity`) _array_element)
    (`LightComponent.SetIntensity` _array_element (* (`LightComponentBase.Intensity` _array_element) _intensitymultiply))
    (`LightComponent.SetLightColor` _array_element (`self.Light Color`) true))
  (`PrimitiveComponent.SetDefaultCustomPrimitiveDataFloat` _lamp 0 (* _intensitymultiply 2.0))
  (`PrimitiveComponent.SetDefaultCustomPrimitiveDataVector4` _lamp 1 (`KismetMathLibrary.MakeVector4` _light_color_r _light_color_g _light_color_b _light_color_a)))