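; BP_Door is an interactable door that swings open or closed each time Interact is called.
; It caches the mesh's current yaw, then a timeline adds or subtracts its rotation curve from that yaw depending on IsOpen.
; A busy flag blocks re-triggering mid-swing, and the open state flips when the timeline finishes.
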(event `self.Interact`
  (bind (_relativerotation_roll _relativerotation_pitch _relativerotation_yaw) (`KismetMathLibrary.BreakRotator` (`SceneComponent.RelativeRotation` (`self.StaticMesh`))))
  (if (not (`self.IsInteract`))
    (set `self.IsInteract` true)
    (set `self.TempYawRotation` _relativerotation_yaw)
    (bind (_direction _rotation) (`Timeline|Timeline` :!via `PlayFromStart`)
      (:`Update`
        (if (`self.IsOpen`)
          (`SceneComponent.K2_SetRelativeRotation` (`self.StaticMesh`) (`KismetMathLibrary.MakeRotator` 0.0 0.0 (+ (* _rotation -1.0) (`self.TempYawRotation`))) false false)
          (else
            (`SceneComponent.K2_SetRelativeRotation` (`self.StaticMesh`) (`KismetMathLibrary.MakeRotator` 0.0 0.0 (+ (* _rotation 1.0) (`self.TempYawRotation`))) false false))))
      (:`Finished`
        (set `self.IsOpen` (not (`self.IsOpen`)))
        (set `self.IsInteract` false)))))

(fn `UserConstructionScript`)